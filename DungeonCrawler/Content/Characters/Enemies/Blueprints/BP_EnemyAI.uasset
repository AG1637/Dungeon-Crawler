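; Enemy character that wanders random navmesh points and chases the player for a melee kick when PawnSensing spots them.
; Tick drives patrol and a health bar widget that faces the camera.
; The kick montage's completion triggers a sphere overlap that damages Player-tagged actors.
; At zero health it ragdolls, spawns wood and sometimes a random pickup at ground-traced nearby points, then destroys itself.
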(event OnSeePawn(PawnSensing)
  (params (Pawn :type Pawn%20Object%20Reference))
  ;[1 1 1] Enemy patrols and then follows player when it can see them
  (Variables|Default|SetIsSeeingPlayer? true)
  (CallFunction|AttackPlayer))

(event Custom|AttackPlayer
  ;[1 1 1] Enemy Attacks Player
  (if (Variables|Default|GetIsSeeingPlayer?)
    (AI|AIMoveTo self "0, 0, 0" (Game|GetPlayerCharacter 0) 85.0 false
      (:OnSuccess
        (if (Variables|Default|GetcanAttack?)
          (Variables|Default|SetcanAttack? false)
          (Animation|Montage|PlayMontage (Variables|Character|GetMesh) "/Game/Characters/Enemies/Animations/ImportedFromMixamo/Kick/NewKick_Montage.NewKick_Montage"
            (:OnCompleted
              (bind _outactors (Collision|SphereOverlapActors (Transformation|GetWorldLocation (Variables|Default|GetArrow1)) 1e+02 (Variables|Default|GetObject%20Types) 0))
              (bind _array_element (Utilities|Array|ForEachLoopwithBreak _outactors)
                (:LoopBody
                  (if (Actor|ActorHasTag _array_element "Player")
                    (Game|Damage|ApplyDamage _array_element 1e+01 0 0)))
                (:Completed
                  (Variables|Default|SetcanAttack? true))))))))
    (else
      (Variables|Default|SetIsSeeingPlayer? false))))

(event Custom|Patrol
  ;[1 1 1] Enemy patrols and then follows player when it can see them
  (if (not (Variables|Default|GetIsSeeingPlayer?))
    (Utilities|FlowControl|Delay (Math|Random|RandomFloatinRange 2.0 5.0))
    (AI|AIMoveTo self (.RandomLocation (AI|Navigation|GetRandomReachablePointinRadius (Transformation|GetActorLocation) 2.5e+03 0 0)) 0 5.0 false
      (:then
        (Variables|Default|SetIsSeeingPlayer? false)))))

(event Custom|SpawnWood
  (bind _returnvalue (Transformation|GetActorLocation))
  ;[1 1 1] Enemy drops loot when killed
  (bind _outhit (Collision|LineTraceByChannel _returnvalue (- _returnvalue "0.000000,0.000000,200.000000") "TraceTypeQuery1" false (Utilities|Array|MakeArray (Game|GetPlayerController 0)) "None"))
  (Game|SpawnActorfromClass "/Game/Collectibles/BP_Wood.BP_Wood_C" (Math|Transform|MakeTransform (+ (.RandomLocation (AI|Navigation|GetRandomReachablePointinRadius (.Location (Collision|BreakHitResult _outhit)) 2e+02 0 0)) "0.000000,0.000000,50.000000") (Math|Rotator|MakeRotator 0.0 0.0 (Math|Random|RandomFloatinRange 0.0 3.6e+02))) "AdjustIfPossibleButDontSpawnIfColliding" "MultiplyWithRoot" 0 0))

(event Custom|EnemyHealthBar
  ;[1 1 1] Enemy health bar always faces camera
  (bind _aswbp_enemy_health (Utilities|Casting|CastToWBP_EnemyHealth (UserInterface|GetWidget (Variables|Default|GetHealth%20Bar%20Widget))))
  (Progress|SetPercent (Variables|/Game/UI/WBP_EnemyHealth.WBP_EnemyHealth_C|GetEnemyHealthBar _aswbp_enemy_health) (/ (Variables|Default|GetHealth) 1e+02))
  (Transformation|SetWorldRotation (Variables|Default|GetHealth%20Bar%20Widget) (Math|Rotator|FindLookatRotation (Transformation|GetWorldLocation (Variables|Default|GetHealth%20Bar%20Widget)) (Transformation|GetWorldLocation (Variables|/Script/Engine.PlayerCameraManager|GetTransformComponent (Game|GetPlayerCameraManager 0)))) false false))

(event Custom|EnemyLootDrop
  (bind _returnvalue (Transformation|GetActorLocation))
  ;[1 1 1] Enemy drops loot when killed
  (bind _outhit (Collision|LineTraceByChannel _returnvalue (- _returnvalue "0.000000,0.000000,200.000000") "TraceTypeQuery1" false (Utilities|Array|MakeArray (Game|GetPlayerController 0)) "None"))
  (Game|SpawnActorfromClass (Utilities|Select :Index (Math|Random|RandomInteger 2) :Option%200 "/Game/Collectibles/BP_HealthBoost.BP_HealthBoost_C" :Option%201 "/Game/Collectibles/BP_SpeedBoost.BP_SpeedBoost_C" :Option%202 "/Game/Collectibles/BP_Wood.BP_Wood_C") (Math|Transform|MakeTransform (+ (.RandomLocation (AI|Navigation|GetRandomReachablePointinRadius (.Location (Collision|BreakHitResult _outhit)) 2e+02 0 0)) "0.000000,0.000000,50.000000") (Math|Rotator|MakeRotator 0.0 0.0 (Math|Random|RandomFloatinRange 0.0 3.6e+02))) "AdjustIfPossibleButDontSpawnIfColliding" "MultiplyWithRoot" 0 0))

(event Game|Damage|EventAnyDamage
  (params (Damage :type Float%20%28single-precision%29) (DamageType :type Damage%20Type%20Object%20Reference) (InstigatedBy :type Controller%20Object%20Reference) (DamageCauser :type Actor%20Object%20Reference))
  ;[1 1 1] Enemy takes damage and dies when health hits zero
  (Variables|Default|SetHealth (- (Variables|Default|GetHealth) Damage))
  (if (<= (Variables|Default|GetHealth) 0.0)
    (Variables|Default|SetSpawnCollectibleNumber (Math|Random|RandomIntegerinRange 0 1))
    (if (== (Variables|Default|GetSpawnCollectibleNumber) 1)
      (CallFunction|EnemyLootDrop)
      (CallFunction|SpawnWood)
      (else
        (CallFunction|SpawnWood)))
    (Physics|SetSimulatePhysics (Variables|Character|GetMesh) true)
    (Utilities|FlowControl|Delay 2.0)
    (Actor|DestroyActor)))

(event EventTick
  (params (DeltaSeconds :type Float%20%28single-precision%29))
  (Utilities|FlowControl|Sequence
    (:then_0
      (CallFunction|Patrol))
    (:then_1
      (CallFunction|EnemyHealthBar))))

(fn ConstructionScript)